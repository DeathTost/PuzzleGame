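; Skeleton enemy character that handles its death state and stores two patrol waypoints.
; The construction script adds two waypoint offsets to the actor's location to produce world-space waypoint vectors.
; Tick polls IsDead and, while it is true, disables movement and actor collision, then starts a five-second delay with nothing connected after it.
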(event EventBeginPlay)

(event Collision|EventActorBeginOverlap
  (params (OtherActor :type Actor%20Object%20Reference)))

(event EventTick
  (params (DeltaSeconds :type Float%20%28single-precision%29))
  (if (Variables|Default|GetIsDead)
    (Pawn|Components|CharacterMovement|DisableMovement (Variables|Character|GetCharacterMovement))
    (Collision|SetActorEnableCollision self false)
    (Utilities|FlowControl|Delay 5.0)))

(fn ConstructionScript
  (bind _returnvalue (Transformation|GetActorLocation))
  (Variables|Default|SetWaypoint_00_Vector (+ _returnvalue (Variables|Default|GetWaypoint_00)))
  (Variables|Default|SetWaypoint_01_Vector (+ _returnvalue (Variables|Default|GetWaypoint_01))))