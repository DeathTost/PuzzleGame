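; Exit door Blueprint that acts as the level's end gate, removing player characters who enter it once it is open.
; OpenVortexEvent activates the particle system and sets IsGameFinished, which arms the overlap box.
; Each PlayerCharacter overlapping the armed box is destroyed, and when none remain in the world it calls AllPlayersKilledEvent on the LevelManager.
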(event OnComponentBeginOverlap(Box)
  (params (OverlappedComponent :type Primitive%20Component%20Object%20Reference) (OtherActor :type Actor%20Object%20Reference) (OtherComp :type Primitive%20Component%20Object%20Reference) (OtherBodyIndex :type Integer) (bFromSweep :type Boolean) (SweepResult :type Hit%20Result%20Structure%20%28by%20ref%29))
  ;[1 1 1] Kill player characters
  (if (Variables|Default|GetIsGameFinished)
    (bind _asplayer_character (Utilities|Casting|CastToPlayerCharacter OtherActor))
    (Actor|DestroyActor _asplayer_character)
    (bind _outactors (Actor|GetAllActorsOfClass "/Game/Animals/PlayerCharacter.PlayerCharacter_C"))
    (if (== (Utilities|Array|Length _outactors) 0)
      (Default|AllPlayersKilledEvent (Variables|Default|GetLevelManager)))))

(event Custom|OpenVortexEvent
  ;[1 1 1] Activate exit gate
  (Components|Activation|Activate (Variables|Default|GetParticleSystem) false)
  (Variables|Default|SetIsGameFinished true))

(fn ConstructionScript)